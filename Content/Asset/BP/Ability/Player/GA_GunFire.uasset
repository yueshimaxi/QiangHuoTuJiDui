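; Player gun-fire Gameplay Ability that launches a projectile from the weapon socket toward a targeted point.
; Activation commits cost and cooldown, then runs a target data task and starts a rifle firing montage.
; An Ability.Fire gameplay event times the shot, which spawns the projectile at the hit location's direction and ends the ability.
; Failed commits never call EndAbility, and debug prints remain throughout.
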(event `self.K2_ActivateAbility`
  (`KismetSystemLibrary.PrintString` "cost")
  (bind _returnvalue (`self.K2_CommitAbilityCost` false))
  (if _returnvalue
    (`KismetSystemLibrary.PrintString` "Hello")
    (bind _returnvalue_2 (`self.K2_CommitAbilityCooldown` false))
    (if _returnvalue_2
      (bind (_asynctaskproxy _data) (`TargetDataTask.CreateTargetDataTask`)
        (:`ValidData`
          (`AbilityTask_PlayMontageAndWait.CreatePlayMontageAndWaitProxy` "None" "/Game/Asset/Anim/BaseShoot/Firing_Rifle__1__Montage.Firing_Rifle__1__Montage" 1.0 "None" false
            (:`then`
              (`AbilityTask_WaitGameplayEvent.WaitGameplayEvent` (struct :`TagName` "Ability.Fire") null
                (:`EventReceived`
                  (`self.SpawnProjectile` (`.Location` (`GameplayStatics.BreakHitResult` (`AbilitySystemBlueprintLibrary.GetHitResultFromTargetData` _data))) (struct :`TagName` "Combat.Socket.Weapon"))
                  (`KismetSystemLibrary.PrintString` "FireBolt Active")
                  (`self.K2_EndAbility`)))))))
      (else
        (`KismetSystemLibrary.PrintString` "Cool Down" _returnvalue_2)))))