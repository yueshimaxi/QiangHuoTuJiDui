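; Player gameplay ability that equips the weapon stored at a given index in the character's combat component.
; On activation it commits, plays the grab-rifle-from-back montage, then sends EquipWeaponMessage with that weapon to the avatar and ends.
; Every montage outcome, including interruption or cancellation, still equips the weapon.
; The cost check override fails when no valid weapon exists at the index, otherwise deferring to the parent check.
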(event `self.K2_ActivateAbility`
  (bind _returnvalue (`self.GetAvatarActorFromActorInfo`))
  (`self.K2_CommitAbility`)
  (if true
    (`AbilityTask_PlayMontageAndWait.CreatePlayMontageAndWaitProxy` "None" "/Game/XuAsset/Anim/BaseShoot/Grab_Rifle_From_Back_Montage.Grab_Rifle_From_Back_Montage"
      (:`OnCompleted`
        _)
      (:`OnBlendOut`
        _)
      (:`OnInterrupted`
        _)
      (:`OnCancelled`
        _))
    (bind _asplayer_character (cast `PlayerCharacter` _returnvalue))
    (bind _returnvalue_2 (`CombatComponent.GetWeaponByIndex` (`PlayerCharacter.combat_component` _asplayer_character) (`self.Index`)))
    (message `PlayerInterface.EquipWeapon` _returnvalue _returnvalue_2)
    (`self.K2_EndAbility`)))

(fn `GSCheckCost`
  (params (Handle :type "GameplayAbilitySpecHandle Structure") (ActorInfo :type "GameplayAbilityActorInfo Structure (by ref)"))
  (returns (ReturnValue :type Boolean))
  (bind _asplayer_character (cast `PlayerCharacter` (`.AvatarActor` (break `GameplayAbilityActorInfo` ActorInfo))))
  (bind _returnvalue (`PlayerCharacter.getCombatCom` _asplayer_character))
  (bind _returnvalue_2 (`CombatComponent.GetWeaponByIndex` _returnvalue (`self.Index`)))
  (`/Engine/EditorBlueprintResources/StandardMacros.IsValid` _returnvalue_2
    (:`Is Valid`
      (return (`parent.GSCheckCost` Handle ActorInfo)))
    (:`Is Not Valid`
      (return false))))