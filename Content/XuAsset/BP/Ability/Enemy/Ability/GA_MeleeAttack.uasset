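; Enemy melee attack gameplay ability that plays a random tagged montage and damages non-friendly actors at the strike point.
; It gets montages and combat target from the avatar via message calls, then waits for the montage's tag event.
; That event triggers a sphere query at the tagged socket, applying damage and firing a MeleeImpact cue on a hit.
; The ability ends when nothing is found or the montage completes, is interrupted or is cancelled.
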(event `self.K2_ActivateAbility`
  (bind _returnvalue (`self.GetAvatarActorFromActorInfo`))
  (bind (_montage _montagetag) (break `TaggedMontage` (`self.tagMontage`)))
  (bind _returnvalue_2 (message `EnemyInterface.GetCombatTarget` _returnvalue))
  (set `self.TargetActor` _returnvalue_2)
  (message `CombatInterface.UpdateFacingTarget` _returnvalue (`Actor.K2_GetActorLocation` (`self.GetAvatarActorFromActorInfo`)))
  (bind _returnvalue_3 (message `CombatInterface.GetTaggedMontages` (`self.GetAvatarActorFromActorInfo`)))
  (bind _returnvalue_4 (`AuraAbilityLibrary.GetRandomTagMotageFromArray` _returnvalue_3))
  (set `self.tagMontage` _returnvalue_4)
  (`AbilityTask_PlayMontageAndWait.CreatePlayMontageAndWaitProxy` "None" _montage
    (:`then`
      (`AbilityTask_WaitGameplayEvent.WaitGameplayEvent` _montagetag null
        (:`EventReceived`
          (bind _returnvalue_5 (message `CombatInterface.GetCombatSocketLocation` (`self.GetAvatarActorFromActorInfo`) (`.SocketTag` (break `TaggedMontage` (`self.tagMontage`)))))
          (bind _output_get (set `self.CombatSocketLocation` _returnvalue_5))
          (bind _outactors (`AuraAbilityLibrary.GetLiveActorOnSphere` _output_get 0.0 (`|MakeArray` (`self.GetAvatarActorFromActorInfo`))))
          (if (> (`KismetArrayLibrary.Array_Length` _outactors) 0)
            (set `self.HasImpact` false)
            (for _array_element _outactors
              (bind _returnvalue_6 (`AuraAbilityLibrary.IsNotFriendly` _array_element (`self.GetAvatarActorFromActorInfo`)))
              (if _returnvalue_6
                (set `self.HasImpact` true)
                (`self.CauseDamage` _array_element)))
            (if (`self.HasImpact`)
              (`self.K2_ExecuteGameplayCueWithParams` (struct :`TagName` "GameplayCue.MeleeImpact") (`AbilitySystemBlueprintLibrary.MakeGameplayCueParameters` 0.0 0.0 (struct) (struct) (struct) (`BlueprintGameplayTagLibrary.MakeGameplayTagContainerFromArray` (`|MakeArray` (`.MontageTag` (break `TaggedMontage` (`self.tagMontage`))))) (struct) (`self.CombatSocketLocation`) (0.0 0.0 0.0) null (`self.GetAvatarActorFromActorInfo`) (`self.TargetActor`))))
            (else
              (`self.K2_EndAbility`))))))
    (:`OnCompleted`
      (`self.K2_EndAbility` :!label _label))
    (:`OnInterrupted`
      (goto _label))
    (:`OnCancelled`
      (goto _label))))