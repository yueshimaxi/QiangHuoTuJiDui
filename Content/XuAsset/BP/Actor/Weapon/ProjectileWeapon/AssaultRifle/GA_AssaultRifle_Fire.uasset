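; Gameplay ability for automatic assault rifle fire, repeating at the current weapon's fire delay until input release or a failed cost check.
; Each shot gets target data, plays the firing montage and spawns a projectile toward the hit location.
; Only with authority, it shakes player 0's camera and executes sound and emitter gameplay cues.
; Cost overrides deduct clip ammo and trigger the reload ability when ammo or the parent check fails.
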(event `self.K2_ActivateAbility`
  (bind _returnvalue (`self.K2_CommitAbility`))
  (if _returnvalue
    (`self.Fire`)
    (`AbilityTask_WaitInputRelease.WaitInputRelease` true
      (:`then`
        (`self.GetFireDelay`)
        (`AbilityTask_WaitDelay.WaitDelay` (`self.Weapon Fire Delay`) :!label _label
          (:`OnFinish`
            (bind _returnvalue_2 (`self.K2_CheckAbilityCost`))
            (if _returnvalue_2
              (`self.K2_CommitAbilityCost` false)
              (`self.Fire`)
              (goto _label)
              (else
                (`self.K2_EndAbility`))))))
      (:`OnRelease`
        (`self.K2_EndAbility`)))
    (else
      (`self.K2_EndAbility`))))

(event `Fire`
  (bind (_asynctaskproxy _data) (`TargetDataTask.CreateTargetDataTask`)
    (:`ValidData`
      (`AbilityTask_PlayMontageAndWait.CreatePlayMontageAndWaitProxy` "None" "/Game/XuAsset/Anim/BaseShoot/Firing_Rifle__1__Montage.Firing_Rifle__1__Montage" 1.0 "None" false
        (:`then`
          (bind (_bblockinghit _binitialoverlap _time _distance _location) (`GameplayStatics.BreakHitResult` (`AbilitySystemBlueprintLibrary.GetHitResultFromTargetData` _data)))
          (`self.SpawnProjectile` _location (struct :`TagName` "Combat.Socket.Weapon"))
          (`self.K2_HasAuthority`
            (:`True`
              (bind _returnvalue (message `CombatInterface.get_cur_projection_weapon` (`self.GetAvatarActorFromActorInfo`)))
              (bind _returnvalue_2 (- _location (`ProjectionWeapon.GetProjectileSpawnLocation` _returnvalue)))
              (`PlayerController.ClientStartCameraShake` (`GameplayStatics.GetPlayerController` 0) "/Game/XuAsset/BP/Ability/Player/CameraShake_GunShoot.CameraShake_GunShoot_C" 1.0 "UserDefined" (`KismetMathLibrary.Conv_VectorToRotator` _returnvalue_2))
              (`self.K2_ExecuteGameplayCueWithParams` (struct :`TagName` "GameplayCue.GunFire.Sound") (`AbilitySystemBlueprintLibrary.MakeGameplayCueParameters` 0.0 0.0 (struct) (struct) (struct) (struct) (struct) (`ProjectionWeapon.GetProjectileSpawnLocation` _returnvalue) (0.0 0.0 0.0) null null (`ProjectionWeapon.FireSound` _returnvalue)))
              (`self.K2_ExecuteGameplayCueWithParams` (struct :`TagName` "GameplayCue.GunFire.Emitter") (`AbilitySystemBlueprintLibrary.MakeGameplayCueParameters` 0.0 0.0 (struct) (struct) (struct) (struct) (struct) (`ProjectionWeapon.GetProjectileSpawnLocation` _returnvalue) _returnvalue_2)))))))))

(event `GetFireDelay`
  (bind _returnvalue (message `CombatInterface.get_cur_projection_weapon` (`self.GetAvatarActorFromActorInfo`)))
  (bind _output_get (set `self.Weapon Fire Delay` (`.weapon_fire_delay` (break `WeaponInfo` (`ProjectionWeapon.weapon_info` _returnvalue)))))
  (`KismetSystemLibrary.PrintString` (`KismetStringLibrary.Conv_DoubleToString` _output_get)))

(fn `GSApplyCost`
  (params (Handle :type "GameplayAbilitySpecHandle Structure") (ActorInfo :type "GameplayAbilityActorInfo Structure (by ref)") (ActivationInfo :type "GameplayAbilityActivationInfo Structure"))
  (bind _returnvalue (message `CombatInterface.get_cur_projection_weapon` (`self.GetAvatarActorFromActorInfo`)))
  (`ProjectionWeapon.SetPrimaryClipAmmo` _returnvalue (- (`ProjectionWeapon.GetPrimaryClipAmmo` _returnvalue) (`self.AmmoCost`)))
  (return))

(fn `GSCheckCost`
  (params (Handle :type "GameplayAbilitySpecHandle Structure") (ActorInfo :type "GameplayAbilityActorInfo Structure (by ref)"))
  (returns (ReturnValue :type Boolean))
  (bind (_owneractor _avataractor _playercontroller _abilitysystemcomponent) (break `GameplayAbilityActorInfo` ActorInfo))
  (bind _returnvalue (message `CombatInterface.get_cur_projection_weapon` _avataractor))
  (if (and (>= (`ProjectionWeapon.GetPrimaryClipAmmo` _returnvalue) (`self.AmmoCost`)) (`parent.GSCheckCost` Handle ActorInfo))
    (return true)
    (else
      (`AbilitySystemComponent.TryActivateAbilitiesByTag` _abilitysystemcomponent (`BlueprintGameplayTagLibrary.MakeGameplayTagContainerFromArray` (`|MakeArray` (struct :`TagName` "Ability.Reload") :!type "GameplayTag Structure")) true)
      (return false))))