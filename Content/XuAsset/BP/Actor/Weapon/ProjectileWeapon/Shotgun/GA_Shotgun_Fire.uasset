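; Gameplay ability that fires a shotgun and keeps firing while the input is held.
; It commits, fires, then repeats after the weapon's fire delay, paying cost each shot and ending on release or when cost fails.
; Each shot uses a shotgun target-data task, plays a montage and spawns a projectile per returned hit.
; With authority, it also triggers camera shake on player 0 and gunfire sound and emitter gameplay cues.
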(event `self.K2_ActivateAbility`
  (bind _returnvalue (`self.K2_CommitAbility`))
  (if _returnvalue
    (`self.Fire`)
    (`AbilityTask_WaitInputRelease.WaitInputRelease` true
      (:`then`
        (`self.GetFireDelay`)
        (`AbilityTask_WaitDelay.WaitDelay` (`self.Weapon Fire Delay`) :!label _label
          (:`OnFinish`
            (bind _returnvalue_2 (`self.K2_CheckAbilityCost`))
            (if _returnvalue_2
              (`self.K2_CommitAbilityCost` false)
              (`self.Fire`)
              (goto _label)
              (else
                (`self.K2_EndAbility`))))))
      (:`OnRelease`
        (`self.K2_EndAbility`)))
    (else
      (`self.K2_EndAbility`))))

(event `Fire`
  (bind (_asynctaskproxy _data) (`ShotgunTargetDataTask.CreateShotgunTargetDataTask` 5)
    (:`ValidData`
      (`AbilityTask_PlayMontageAndWait.CreatePlayMontageAndWaitProxy` "None" "/Game/XuAsset/Anim/BaseShoot/Firing_Rifle__1__Montage.Firing_Rifle__1__Montage" 1.0 "None" false
        (:`then`
          (for _index (range (`AbilitySystemBlueprintLibrary.GetDataCountFromTargetData` _data))
            (bind (_bblockinghit _binitialoverlap _time _distance _location) (`GameplayStatics.BreakHitResult` (`AbilitySystemBlueprintLibrary.GetHitResultFromTargetData` _data _index)))
            (`self.SpawnProjectile` _location (struct :`TagName` "Combat.Socket.Weapon")))
          (`self.K2_HasAuthority`
            (:`True`
              (bind _returnvalue (message `CombatInterface.get_cur_projection_weapon` (`self.GetAvatarActorFromActorInfo`)))
              (bind _returnvalue_2 (- _location (`ProjectionWeapon.GetProjectileSpawnLocation` _returnvalue)))
              (`PlayerController.ClientStartCameraShake` (`GameplayStatics.GetPlayerController` 0) "/Game/XuAsset/BP/Ability/Player/CameraShake_GunShoot.CameraShake_GunShoot_C" 1.0 "UserDefined" (`KismetMathLibrary.Conv_VectorToRotator` _returnvalue_2))
              (`self.K2_ExecuteGameplayCueWithParams` (struct :`TagName` "GameplayCue.GunFire.Sound") (`AbilitySystemBlueprintLibrary.MakeGameplayCueParameters` 0.0 0.0 (struct) (struct) (struct) (struct) (struct) (`ProjectionWeapon.GetProjectileSpawnLocation` _returnvalue) (0.0 0.0 0.0) null null (`ProjectionWeapon.FireSound` _returnvalue)))
              (`self.K2_ExecuteGameplayCueWithParams` (struct :`TagName` "GameplayCue.GunFire.Emitter") (`AbilitySystemBlueprintLibrary.MakeGameplayCueParameters` 0.0 0.0 (struct) (struct) (struct) (struct) (struct) (`ProjectionWeapon.GetProjectileSpawnLocation` _returnvalue) _returnvalue_2)))))))))

(event `GetFireDelay`
  (bind _returnvalue (message `CombatInterface.get_cur_projection_weapon` (`self.GetAvatarActorFromActorInfo`)))
  (bind _output_get (set `self.Weapon Fire Delay` (`.weapon_fire_delay` (break `WeaponInfo` (`ProjectionWeapon.weapon_info` _returnvalue)))))
  (`KismetSystemLibrary.PrintString` (`KismetStringLibrary.Conv_DoubleToString` _output_get)))