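; Gameplay ability that fires the pistol, launching a projectile at the targeted location.
; On activation it commits, gets a hit location from a TargetData task, starts the firing montage and spawns the projectile from the weapon socket.
; On authority only, it shakes player 0's camera, executes sound and muzzle-flash gameplay cues using the current weapon's data, then ends.
; An unconnected SetByCaller cooldown snippet never runs.
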(event `self.K2_ActivateAbility`
  (`self.K2_CommitAbility`)
  (if true
    (bind (_asynctaskproxy _data) (`TargetDataTask.CreateTargetDataTask`)
      (:`ValidData`
        (`AbilityTask_PlayMontageAndWait.CreatePlayMontageAndWaitProxy` "None" "/Game/XuAsset/Anim/BaseShoot/Firing_Rifle__1__Montage.Firing_Rifle__1__Montage" 1.0 "None" false
          (:`then`
            (bind (_bblockinghit _binitialoverlap _time _distance _location) (`GameplayStatics.BreakHitResult` (`AbilitySystemBlueprintLibrary.GetHitResultFromTargetData` _data)))
            (`self.SpawnProjectile` _location (struct :`TagName` "Combat.Socket.Weapon"))
            (`self.K2_HasAuthority`
              (:`True`
                (bind _returnvalue (message `CombatInterface.get_cur_projection_weapon` (`self.GetAvatarActorFromActorInfo`)))
                (bind _returnvalue_2 (- _location (`ProjectionWeapon.GetProjectileSpawnLocation` _returnvalue)))
                (`PlayerController.ClientStartCameraShake` (`GameplayStatics.GetPlayerController` 0) "/Game/XuAsset/BP/Ability/Player/CameraShake_GunShoot.CameraShake_GunShoot_C" 1.0 "UserDefined" (`KismetMathLibrary.Conv_VectorToRotator` _returnvalue_2))
                (`self.K2_ExecuteGameplayCueWithParams` (struct :`TagName` "GameplayCue.GunFire.Sound") (`AbilitySystemBlueprintLibrary.MakeGameplayCueParameters` 0.0 0.0 (struct) (struct) (struct) (struct) (struct) (`ProjectionWeapon.GetProjectileSpawnLocation` _returnvalue) (0.0 0.0 0.0) null null (`ProjectionWeapon.FireSound` _returnvalue)))
                (`self.K2_ExecuteGameplayCueWithParams` (struct :`TagName` "GameplayCue.GunFire.Emitter") (`AbilitySystemBlueprintLibrary.MakeGameplayCueParameters` 0.0 0.0 (struct) (struct) (struct) (struct) (struct) (`ProjectionWeapon.GetProjectileSpawnLocation` _returnvalue) _returnvalue_2 null null (`ProjectionWeapon.MuzzleFlashEffect` _returnvalue)))
                (`self.K2_EndAbility`)))))))))