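; BP_HPBag is an interactable health pickup that reports its type as the Interact.Prop.HPBag tag.
; On interaction it applies a configurable GameplayEffect to the player's Ability System Component and plays a 2D pickup sound.
; It then hides its mesh and disables collision, restoring both after a ReSpawnTime delay so the same actor respawns in place rather than being destroyed.
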(event `self.Interaction`
  (params (playerCharacter :type "PlayerCharacter Object Reference"))
  (bind _staticmesh (`self.StaticMesh`))
  (bind _staticmesh_2 (`self.StaticMesh`))
  (`AbilitySystemComponent.BP_ApplyGameplayEffectToSelf` (`AbilitySystemBlueprintLibrary.GetAbilitySystemComponent` playerCharacter) (`self.GE`) 1.0 (make `GameplayEffectContextHandle`))
  (`GameplayStatics.PlaySound2D` (`self.PickSound`) 1.0 1.0 0.0 null null)
  (`PrimitiveComponent.SetCollisionEnabled` _staticmesh_2 "NoCollision")
  (`SceneComponent.SetHiddenInGame` _staticmesh_2 true false)
  (`KismetSystemLibrary.Delay` (`KismetMathLibrary.Conv_IntToDouble` (`self.ReSpawnTime`)))
  (`SceneComponent.SetHiddenInGame` _staticmesh false false)
  (`PrimitiveComponent.SetCollisionEnabled` _staticmesh "QueryAndPhysics"))

(fn `GetInteractionType`
  (returns (ReturnValue :type "GameplayTag Structure"))
  (return (struct :`TagName` "Interact.Prop.HPBag")))

(fn `UserConstructionScript`)